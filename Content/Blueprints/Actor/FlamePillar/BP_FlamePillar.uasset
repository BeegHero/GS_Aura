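; Flame pillar actor that flickers its fire light continuously from BeginPlay.
; It randomly picks one of two flame intensity timelines and chooses again whenever one finishes, so the flicker pattern varies.
; Each timeline update scales the light's base intensity by the curve value.
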(event Custom|CustomEvent_2
  (bind _flameintensity (Timeline|FlameIntensity_2 PlayFromStart)
    (:Update
      (CallFunction|ScaleFlameIntensity _flameintensity))
    (:Finished
      (CallFunction|ChooseTimeline))))

(event Custom|CustomEvent_1
  (bind _flameintensity (Timeline|FlameIntensity_1 PlayFromStart)
    (:Update
      (CallFunction|ScaleFlameIntensity _flameintensity))
    (:Finished
      (CallFunction|ChooseTimeline))))

(event Custom|ChooseTimeline
  (switch int (Math|Random|RandomIntegerinRange 0 1)
    (:Default
      (CallFunction|CustomEvent1 :!label _label))
    (:0
      (goto _label))
    (:1
      (CallFunction|CustomEvent2))))

(event EventBeginPlay
  (CallFunction|ChooseTimeline))

(fn ConstructionScript)

(fn ScaleFlameIntensity
  (params (Percentage :type Float%20%28double-precision%29))
  (Rendering|Components|Light|SetIntensity (Variables|Default|GetFireLight) (* Percentage (Variables|Default|GetBaseIntensity))))